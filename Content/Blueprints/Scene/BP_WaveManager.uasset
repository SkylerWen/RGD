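; BP_WaveManager is a placed enemy generator that spawns successive waves of enemies around its own location, starting at BeginPlay.
; Each wave's enemy groups set class, level and count, with spawns randomly scattered horizontally and tracked in ActiveEnemies.
; Destroyed-event bindings empty that list, triggering the next wave after a short delay.
; After the last wave, it reports to BP_LevelManager that this generator finished, then destroys itself.
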(event `self.ReceiveBeginPlay`
  (if (< (`self.CurrentWaveIndex`) (`KismetArrayLibrary.Array_Length` (`self.AllWaves`)))
    (`self.SpawnNextWave`)))

(event `SpawnNextWave`
  (bind _returnvalue_location (`KismetMathLibrary.BreakTransform` (`self.GetTransform`)))
  (bind _output_enemygroups (break `/Game/Atomics/ST_WaveConfig` (`|GetArrayItem` (`self.AllWaves`) (`self.CurrentWaveIndex`))))
  (for _array_element _output_enemygroups
    (for _ (range 1 (+ (`.Count_7_35C839244B0D1C1E7F93E0AA59DD4D26` (break `/Game/Atomics/ST_SpawnGroup` _array_element)) 1))
      (bind _returnvalue (`|SpawnActorFromClass` (break `/Game/Atomics/ST_SpawnGroup` _array_element) (`KismetMathLibrary.MakeTransform` (+ _returnvalue_location (`KismetMathLibrary.MakeVector` (`KismetMathLibrary.RandomFloatInRange` -150.0 150.0) (`KismetMathLibrary.RandomFloatInRange` -150.0 150.0)))) "Undefined" "MultiplyWithRoot" null (`.Level_8_1F8DA6A74ED37BF03A6D7F9D09E048B5` (break `/Game/Atomics/ST_SpawnGroup` _array_element)) null))
      (`KismetArrayLibrary.Array_AddUnique` (`self.ActiveEnemies`) _returnvalue)
      (add `self.OnDestroyed` _returnvalue (delegate `HandleEnemyDeath`)))))

(event `HandleEnemyDeath` :!signature `self.OnDestroyed`
  (params (DestroyedActor :type "Actor Object Reference"))
  (bind _asbp_enemy_base (cast `/Game/Blueprints/Enemy/BP_EnemyBase` DestroyedActor))
  (`KismetArrayLibrary.Array_RemoveItem` (`self.ActiveEnemies`) _asbp_enemy_base)
  (if (== (`KismetArrayLibrary.Array_Length` (`self.ActiveEnemies`)) 0)
    (`KismetSystemLibrary.Delay` 1.0)
    (set `self.CurrentWaveIndex` (+ (`self.CurrentWaveIndex`) 1))
    (if (< (`self.CurrentWaveIndex`) (`KismetArrayLibrary.Array_Length` (`self.AllWaves`)))
      (`self.SpawnNextWave`)
      (else
        (bind _returnvalue (`GameplayStatics.GetActorOfClass` "/Game/Blueprints/Scene/BP_LevelManager.BP_LevelManager_C"))
        (`/Game/Blueprints/Scene/BP_LevelManager.Report Generator Finished` _returnvalue)
        (`self.K2_DestroyActor`)))))

(fn `UserConstructionScript`)