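; BP_LevelManager tracks wave completion in a level and loads the next level when every wave manager is done.
; On BeginPlay it counts the BP_WaveManager actors in the level as active generators.
; Each ReportGeneratorFinished call decrements that count, and once it reaches zero or below, it opens NextLevelName after a short delay.
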(event `self.ReceiveBeginPlay`
  (bind _outactors (`GameplayStatics.GetAllActorsOfClass` "/Game/Blueprints/Scene/BP_WaveManager.BP_WaveManager_C"))
  (set `self.ActiveGenerators` (`KismetArrayLibrary.Array_Length` _outactors)))

(event `Report Generator Finished`
  (set `self.ActiveGenerators` (- (`self.ActiveGenerators`) 1))
  (if (<= (`self.ActiveGenerators`) 0)
    (`KismetSystemLibrary.Delay` 2.0)
    (`GameplayStatics.OpenLevel` (`self.NextLevelName`))))

(fn `UserConstructionScript`)