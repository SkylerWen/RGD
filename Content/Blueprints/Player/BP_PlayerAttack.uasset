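; BP_PlayerAttack is a player attack projectile that deals melee damage to enemies on overlap.
; Its Sphere overlap reacts only to actors tagged Destroy, using AuraLevel as the row name to look up DT_PlayerAtomics.
; When the row is found, actors also tagged Enemy take that row's MeleeDamage, then the projectile stops and destroys itself whether or not damage was applied.
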(event `self.Sphere.OnComponentBeginOverlap`
  (params (OverlappedComponent :type "PrimitiveComponent Object Reference") (OtherActor :type "Actor Object Reference") (OtherComp :type "PrimitiveComponent Object Reference") (OtherBodyIndex :type Integer) (bFromSweep :type Boolean) (SweepResult :type "HitResult Structure (by ref)"))
  ; Apply Damage
  (if (`self.ActorHasTag` OtherActor "Destroy")
    (bind _returnvalue (`|GetDataTableRow` "/Game/Atomics/DT_PlayerAtomics.DT_PlayerAtomics" (`KismetStringLibrary.Conv_StringToName` (`KismetStringLibrary.Conv_IntToString` (`self.AuraLevel`))))
      (:`then`
        (if (`self.ActorHasTag` OtherActor "Enemy")
          (`GameplayStatics.ApplyDamage` OtherActor (break `/Game/Atomics/ST_PlayerAtomics` _returnvalue)))
        (`MovementComponent.StopMovementImmediately` (`self.ProjectileMovement`))
        (`self.K2_DestroyActor`)))))

(fn `UserConstructionScript`)