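; BP_Experience is an XP essence pickup that the player character collects in the top-down game.
; When the character enters MagnetRadius, the pickup stores it as a target and interpolates toward it every Tick.
; When Sphere overlaps the player's capsule, it reads XPValue from its MyRowName row in DT_EssenceDrops, passes it to AddXP and destroys itself.
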(event `self.Sphere.OnComponentBeginOverlap`
  (params (OverlappedComponent :type "PrimitiveComponent Object Reference") (OtherActor :type "Actor Object Reference") (OtherComp :type "PrimitiveComponent Object Reference") (OtherBodyIndex :type Integer) (bFromSweep :type Boolean) (SweepResult :type "HitResult Structure (by ref)"))
  (bind _asbp_top_down_char (cast `/Game/Blueprints/Player/BP_TopDownChar` (`GameplayStatics.GetPlayerCharacter` 0)))
  (if (== OtherComp (`Character.CapsuleComponent` _asbp_top_down_char))
    (bind _returnvalue (`|GetDataTableRow` "/Game/Atomics/DT_EssenceDrops.DT_EssenceDrops" (`self.MyRowName`))
      (:`then`
        (`/Game/Blueprints/Player/BP_TopDownChar.AddXP` _asbp_top_down_char (break `/Game/Atomics/ST_EssenceData` _returnvalue))
        (`self.K2_DestroyActor`)))))

(event `self.MagnetRadius.OnComponentBeginOverlap`
  (params (OverlappedComponent :type "PrimitiveComponent Object Reference") (OtherActor :type "Actor Object Reference") (OtherComp :type "PrimitiveComponent Object Reference") (OtherBodyIndex :type Integer) (bFromSweep :type Boolean) (SweepResult :type "HitResult Structure (by ref)"))
  (bind _asbp_top_down_char (cast `/Game/Blueprints/Player/BP_TopDownChar` OtherActor))
  (set `self.TargetPlayer` _asbp_top_down_char)
  (set `self.IsFlying` true))

(event `self.ReceiveTick`
  (params (DeltaSeconds :type "Float (single-precision)"))
  (if (`self.IsFlying`)
    (`self.K2_SetActorLocation` (`KismetMathLibrary.VInterpTo` (`self.K2_GetActorLocation`) (`self.K2_GetActorLocation` (`self.TargetPlayer`)) DeltaSeconds 8.0))))

(fn `UserConstructionScript`)