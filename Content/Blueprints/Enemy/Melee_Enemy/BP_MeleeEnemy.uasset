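; BP_MeleeEnemy is a melee enemy that chases player 0 along the X or Y axis and enters an attack state at close range.
; Each Tick moves it along one axis, switching only when the other distance leads by a margin to prevent jitter.
; It updates IsMoving and a four-way Directionality with inverted Y.
; Within range, it stops adding input and raises IsAttacking for a timed delay, without applying damage here.
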(event `self.ReceiveTick`
  (params (DeltaSeconds :type "Float (single-precision)"))
  (bind (_returnvalue_x _returnvalue_y) (`KismetMathLibrary.BreakVector` (- (`self.K2_GetActorLocation` (`GameplayStatics.GetPlayerCharacter` 0)) (`self.K2_GetActorLocation`))))
  (bind _returnvalue (`KismetMathLibrary.Abs` _returnvalue_x))
  (bind _returnvalue_2 (`KismetMathLibrary.Abs` _returnvalue_y))
  (set `self.IsMoving` (> (`KismetMathLibrary.VSize` (`self.GetVelocity`)) 5.0))
  (if (> (`self.GetDistanceTo` (`GameplayStatics.GetPlayerCharacter` 0)) 300.0)
    ; Move
    (if (`self.IsMovingHorizontal`)
      (if (> _returnvalue_2 (+ _returnvalue 150.0))
        (set `self.IsMovingHorizontal` false))
      (elif (> _returnvalue (+ _returnvalue_2 150.0))
        (set `self.IsMovingHorizontal` true)))
    (if (`self.IsMovingHorizontal`)
      (if (> _returnvalue_x 0.0)
        (`self.AddMovementInput` (1.0 0.0 0.0))
        (set `self.Directionality` (1.0 0.0))
        (else
          (`self.AddMovementInput` (-1.0 0.0 0.0))
          (set `self.Directionality` (-1.0 0.0))))
      (elif (> _returnvalue_y 0.0)
        (`self.AddMovementInput` (0.0 1.0 0.0))
        (set `self.Directionality` (0.0 -1.0))
        (else
          (`self.AddMovementInput` (0.0 -1.0 0.0))
          (set `self.Directionality` (0.0 1.0)))))
    (else
      ; Set attack
      (if (not (`self.IsAttacking`))
        (set `self.IsAttacking` true)
        (`KismetSystemLibrary.Delay` 0.8)
        (set `self.IsAttacking` false)))))

(fn `UserConstructionScript`)