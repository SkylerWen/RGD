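; Dash enemy that chases the player in a top-down game and launches itself at them when close.
; Tick moves it along one axis at a time with hysteresis, setting Directionality, then runs a delayed wind-up, launch, stop and recovery.
; DT_DashEnemy supplies stats by VariantLevel, though timings are hardcoded and DashCooldown is unused here.
; HitBox overlaps deal damage while attacking; BPHealth drives the health bar and death, which spawns BP_Experience.
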(event `self.ReceiveTick`
  (params (DeltaSeconds :type "Float (single-precision)"))
  (bind (_returnvalue_x _returnvalue_y) (`KismetMathLibrary.BreakVector` (- (`self.K2_GetActorLocation` (`GameplayStatics.GetPlayerCharacter` 0)) (`self.K2_GetActorLocation`))))
  (bind (_returnvalue_x_2 _returnvalue_y_2) (`KismetMathLibrary.BreakVector` (- (`self.K2_GetActorLocation` (`GameplayStatics.GetPlayerCharacter` 0)) (`self.K2_GetActorLocation`))))
  (bind _returnvalue (`KismetMathLibrary.Abs` _returnvalue_y_2))
  (bind _returnvalue_2 (`KismetMathLibrary.Abs` _returnvalue_x_2))
  (if (not (`self.IsAttacking`))
    (set `self.IsMoving` (> (`KismetMathLibrary.VSize` (`self.GetVelocity`)) 5.0))
    (if (> (`self.GetDistanceTo` (`GameplayStatics.GetPlayerCharacter` 0)) 500.0)
      ; Move
      (if (`self.IsMovingHorizontal`)
        (if (> _returnvalue (+ _returnvalue_2 150.0))
          (set `self.IsMovingHorizontal` false))
        (elif (> _returnvalue_2 (+ _returnvalue 150.0))
          (set `self.IsMovingHorizontal` true)))
      (if (`self.IsMovingHorizontal`)
        (if (> _returnvalue_x_2 0.0)
          (`self.AddMovementInput` (1.0 0.0 0.0))
          (set `self.Directionality` (1.0 0.0))
          (else
            (`self.AddMovementInput` (-1.0 0.0 0.0))
            (set `self.Directionality` (-1.0 0.0))))
        (elif (> _returnvalue_y_2 0.0)
          (`self.AddMovementInput` (0.0 1.0 0.0))
          (set `self.Directionality` (0.0 -1.0))
          (else
            (`self.AddMovementInput` (0.0 -1.0 0.0))
            (set `self.Directionality` (0.0 1.0)))))
      (else
        ; Dash
        (if (not (`self.IsAttacking`))
          (set `self.IsAttacking` true)
          (if (> (`KismetMathLibrary.Abs` _returnvalue_x) (`KismetMathLibrary.Abs` _returnvalue_y))
            (if (> _returnvalue_x 0.0)
              (set `self.Directionality` (1.0 0.0))
              (else
                (set `self.Directionality` (-1.0 0.0))))
            (elif (> _returnvalue_y 0.0)
              (set `self.Directionality` (0.0 -1.0))
              (else
                (set `self.Directionality` (0.0 1.0)))))
          (`KismetSystemLibrary.Delay` 0.8)
          (`self.LaunchCharacter` (* (`KismetMathLibrary.Normal` (- (`self.K2_GetActorLocation` (`GameplayStatics.GetPlayerCharacter` 0)) (`self.K2_GetActorLocation`))) (`self.Dash Distance`)) true true)
          (`KismetSystemLibrary.Delay` 0.25)
          (`MovementComponent.StopMovementImmediately` (`self.CharacterMovement`))
          (`KismetSystemLibrary.Delay` 1.0)
          (set `self.IsAttacking` false))))))

(event `self.ReceiveBeginPlay`
  (bind _bp_health (`self.BP_Health`))
  ; BeginPlay
  (bind _returnvalue (`|GetDataTableRow` "/Game/Atomics/DT_DashEnemy.DT_DashEnemy" (`KismetStringLibrary.Conv_StringToName` (`KismetStringLibrary.Conv_IntToString` (`self.VariantLevel`))))
    (:`then`
      (bind _output_get (set `/Game/Blueprints/BP_Health.MaxHealth` (break `/Game/Atomics/ST_DashEnemy` _returnvalue) _bp_health))
      (bind _output_get_2 (set `/Game/Blueprints/BP_Health.CurrentHealth` _output_get _bp_health))
      (bind _aswbp_enemy_health_bar (cast `/Game/UI/WBP_EnemyHealthBar` (`WidgetComponent.GetUserWidgetObject` (`self.Widget`))))
      (`/Game/UI/WBP_EnemyHealthBar.UpdateHPBar` _aswbp_enemy_health_bar _output_get_2 _output_get_2)
      (set `self.Dash Cooldown` (`.AttackCooldown_18_B0361EEF4A44592A037974B0621CB70B` (break `/Game/Atomics/ST_DashEnemy` _returnvalue)))
      (set `self.Dash Damage` (`.DashDamage_17_24C430D8435DA4C083A1F7BDE962AA6E` (break `/Game/Atomics/ST_DashEnemy` _returnvalue)))
      (set `self.Dash Distance` (`.DashDistance_23_95A8C6684FD5A7F3B0E07E8357F00ED9` (break `/Game/Atomics/ST_DashEnemy` _returnvalue))))))

(event `self.BP_Health.OnHealthChanged`
  (params (NewHealth :type "Float (double-precision)") (MaxHealth :type "Float (double-precision)"))
  ; Health Change
  (bind _aswbp_enemy_health_bar (cast `/Game/UI/WBP_EnemyHealthBar` (`WidgetComponent.GetUserWidgetObject` (`self.Widget`))))
  (`/Game/UI/WBP_EnemyHealthBar.UpdateHPBar` _aswbp_enemy_health_bar NewHealth MaxHealth))

(event `self.ReceiveAnyDamage`
  (params (Damage :type "Float (single-precision)") (DamageType :type "DamageType Object Reference") (InstigatedBy :type "Controller Object Reference") (DamageCauser :type "Actor Object Reference"))
  ; Apply Damage
  (`/Game/Blueprints/BP_Health.ChangeHealth_Event` (`self.BP_Health`) (* Damage -1.0)))

(event `self.HitBox.OnComponentBeginOverlap`
  (params (OverlappedComponent :type "PrimitiveComponent Object Reference") (OtherActor :type "Actor Object Reference") (OtherComp :type "PrimitiveComponent Object Reference") (OtherBodyIndex :type Integer) (bFromSweep :type Boolean) (SweepResult :type "HitResult Structure (by ref)"))
  ; Attack Apply Damage
  (bind _asbp_top_down_char (cast `/Game/Blueprints/Player/BP_TopDownChar` OtherActor))
  (if (`self.IsAttacking`)
    (`GameplayStatics.ApplyDamage` _asbp_top_down_char (`self.Dash Damage`) null self)))

(event `self.BP_Health.OnDeath`
  ; On Death
  (`self.K2_DestroyActor`)
  (`|SpawnActorFromClass` "/Game/Blueprints/Player/BP_Experience.BP_Experience_C" (`self.GetTransform`) "Undefined" "MultiplyWithRoot" null (`KismetStringLibrary.Conv_StringToName` (`KismetStringLibrary.Concat_StrStr` (`KismetStringLibrary.Conv_NameToString` (`self.EnemyID`)) "_" (`KismetStringLibrary.Conv_IntToString` (`self.VariantLevel`)))) null))

(fn `UserConstructionScript`)