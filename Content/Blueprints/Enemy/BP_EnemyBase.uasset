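; BP_EnemyBase is an enemy base Blueprint using a sprite and PaperZD animation.
; On BeginPlay it tints the sprite with its Color variable.
; Attack jumps the animation instance to the Attack node unless the current sequence's display name is already "Attack", so the attack does not restart.
; ChooseNewDirection is an empty event in this class.
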(event `self.ReceiveBeginPlay`
  (`PaperFlipbookComponent.SetSpriteColor` (`self.Sprite`) (`self.Color`)))

(event `ChooseNewDirection`)

(fn `Attack`
  (if (not (`KismetStringLibrary.EqualEqual_StrStr` (`KismetSystemLibrary.GetDisplayName` (`PaperZDAnimPlayer.GetCurrentAnimSequence` (`PaperZDAnimInstance.GetPlayer` (`PaperZDAnimationComponent.AnimInstance` (`self.AnimationComponent`))))) "Attack"))
    (`PaperZDAnimInstance.JumpToNode` (`PaperZDAnimationComponent.AnimInstance` (`self.AnimationComponent`)) "Attack" "None")))

(fn `UserConstructionScript`)