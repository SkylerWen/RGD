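; BP_Health tracks an owner's health, starting CurrentHealth at MaxHealth on BeginPlay.
; ChangeHealth_Event takes a signed amount to heal or damage, clamping the result between zero and the maximum.
; Each change broadcasts OnHealthChanged with current and max health, then OnDeath whenever health is at zero, with no guard against repeat death calls.
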(event `self.ReceiveBeginPlay`
  ; BeginPlay
  (set `self.CurrentHealth` (`self.MaxHealth`)))

(event `ChangeHealth_Event`
  (params (Amount :type "Float (double-precision)"))
  ; Change HP : A positive Amount value restores HP; a negative Amount value reduces HP
  (bind _output_get (set `self.CurrentHealth` (`KismetMathLibrary.FClamp` (+ (`self.CurrentHealth`) Amount) 0.0 (`self.MaxHealth`))))
  (`self.OnHealthChanged` _output_get (`self.MaxHealth`))
  (if (<= (`self.CurrentHealth`) 0.0)
    (`self.OnDeath`)))